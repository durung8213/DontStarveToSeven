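; BP_HKTPlayer is a player Blueprint with debug keys for testing enemy AI, hearing and boss damage.
; Key 1 toggles an enemy's AI controller between attacking and passive; F makes noise with explosion effects.
; X calls MultiX to explode and damage the first boss; ServerX is never run.
; TakeDamage lowers health, but its clamped check always sets IsDead; getters expose health, death and zeroed ideal ranges.
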(event `self.ReceiveBeginPlay`
  (bind _returnvalue (`GameplayStatics.GetActorOfClass` "/Game/Hamkt/Enemy/BP_BossFirst.BP_BossFirst_C"))
  (set `self.BP_FirstBoss` _returnvalue))

(event `Key|One`
  (params (Key :type "Key Structure"))
  ;[1 1 1] 1번키로 몬스터의 상태를 변화
  (:`Pressed`
    (bind _returnvalue (`GameplayStatics.GetActorOfClass` "/Game/Hamkt/Enemy/BP_EnemyBase.BP_EnemyBase_C"))
    (bind _asaic_enemy_base (cast `AIC_EnemyBase` (`AIBlueprintHelperLibrary.GetAIController` _returnvalue)))
    (`/Engine/EditorBlueprintResources/StandardMacros.FlipFlop`
      (:`A`
        (`AIC_EnemyBase.SetStateAsAttacking` _asaic_enemy_base self))
      (:`B`
        (`AIC_EnemyBase.SetStateAsPassive` _asaic_enemy_base)))))

(event `Key|F`
  (params (Key :type "Key Structure"))
  (bind _returnvalue (`self.K2_GetActorLocation`))
  ;[1 1 1] 청각 테스트 F키
  (:`Pressed`
    (`self.MakeNoise` 1.0 self _returnvalue)
    (`GameplayStatics.SpawnEmitterAtLocation` "/Game/StarterContent/Particles/P_Explosion.P_Explosion" _returnvalue)
    (`GameplayStatics.PlaySoundAtLocation` "/Game/Assets/StarterContent/Audio/Explosion_Cue.Explosion_Cue" _returnvalue (struct) 1.0 1.0 0.0 null null null null)))

(event `MultiX`
  (bind _returnvalue (`GameplayStatics.GetActorOfClass` "/Game/Hamkt/Enemy/Boss/BP_EnemyBossFirst.BP_EnemyBossFirst_C"))
  (`GameplayStatics.SpawnEmitterAtLocation` "/Game/StarterContent/Particles/P_Explosion.P_Explosion" (`self.K2_GetActorLocation` _returnvalue))
  (`BPI_EnemyAI.TakeDamage` _returnvalue 20.0))

(event `Key|X`
  (params (Key :type "Key Structure"))
  (:`Pressed`
    (`self.MultiX`)))

(event `self.TakeDamage`
  (params (Amount :type "Float (single-precision)"))
  (bind _output_get (set `self.CurrentHealth` (- (`self.CurrentHealth`) Amount)))
  (if (<= 0.0 (`KismetMathLibrary.FClamp` _output_get 0.0 100.0))
    (set `self.bIsDead` true)))

(fn `GetCurrentHealth`
  (returns (ReturnValue :type "Float (single-precision)"))
  (return (`self.CurrentHealth`)))

(fn `GetIdealRange`
  (returns (AttackRadius :type "Float (single-precision)") (DefendRadius :type "Float (single-precision)"))
  (return 0.0 0.0))

(fn `GetMaxHealth`
  (returns (ReturnValue :type "Float (single-precision)"))
  (return (`self.MaxHealth`)))

(fn `IsDead`
  (returns (ReturnValue :type Boolean))
  (return (`self.bIsDead`)))

(fn `UserConstructionScript`)