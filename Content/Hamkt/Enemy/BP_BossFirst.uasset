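; BP_BossFirst is a boss enemy Blueprint that plays the montages for waking, attacking and dying.
; Events trigger a roar, two standard attacks, a jump attack, a forward bite and death, all slightly slowed.
; All but death fire a matching dispatcher when the montage completes or is interrupted, signalling the action's end.
; BeginPlay caches the player, unused here, and the attacks' notify switches have no logic attached.
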(event `self.ReceiveBeginPlay`
  (bind _returnvalue (`GameplayStatics.GetActorOfClass` "/Game/Hamkt/Player/BP_HKTPlayer.BP_HKTPlayer_C"))
  (set `self.BP_Player` _returnvalue))

(event `WakeUp`
  ;[1 1 1] Comment
  (`|PlayMontage` (`self.Mesh`) (`self.AM_Roar`) 0.8
    (:`OnCompleted`
      _)
    (:`OnInterrupted`
      _))
  (`self.OnWakeUp`))

(event `Attack1`
  (bind _notifyname (`|PlayMontage` (`self.Mesh`) (`self.AM_Attack1`) 0.8)
    (:`OnCompleted`
      (`self.OnAttack1` :!label _label))
    (:`OnInterrupted`
      (goto _label))
    (:`OnNotifyBegin`
      (switch `name` _notifyname))))

(event `Attack2`
  (bind _notifyname (`|PlayMontage` (`self.Mesh`) (`self.AM_Attack2`) 0.8)
    (:`OnCompleted`
      (`self.OnAttack2` :!label _label_2))
    (:`OnInterrupted`
      (goto _label_2))
    (:`OnNotifyBegin`
      (switch `name` _notifyname))))

(event `JumpAttack`
  (bind _notifyname (`|PlayMontage` (`self.Mesh`) (`self.AM_JumpAttack`) 0.8)
    (:`OnCompleted`
      (`self.OnJumpAttack` :!label _label_3))
    (:`OnInterrupted`
      (goto _label_3))
    (:`OnNotifyBegin`
      (switch `name` _notifyname))))

(event `BiteFoward`
  (bind _notifyname (`|PlayMontage` (`self.Mesh`) (`self.AM_BiteForward`) 0.8)
    (:`OnCompleted`
      (`self.OnBiteForwardAttack` :!label _label_4))
    (:`OnInterrupted`
      (goto _label_4))
    (:`OnNotifyBegin`
      (switch `name` _notifyname))))

(event `Death`
  (`|PlayMontage` (`self.Mesh`) (`self.AM_Death`) 0.8))

(fn `UserConstructionScript`
  (`parent.UserConstructionScript`))