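; BP_MonsterSpawnPoint is a spawn point actor that spawns monsters at its own transform on a repeating timer.
; On BeginPlay the server starts the looping timer, and each spawn prints the actor's name and increments a counter.
; At the third spawn the class switches to BP_EnemyRange.
; The fifth-spawn timer clear is nested inside that third-spawn check, so it never runs.
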(event `self.ReceiveBeginPlay`
  (`/Engine/EditorBlueprintResources/ActorMacros.Switch Has Authority`
    (:`Authority`
      (bind _returnvalue (`KismetSystemLibrary.K2_SetTimerDelegate` (`|CreateDelegate` :!event `SpawnEvent`) (`self.Time`) true))
      (set `self.TH_MonsterTimerHandle` _returnvalue))))

(event `SpawnEvent`
  (bind _returnvalue (`|SpawnActorFromClass` (`self.Class`) (`self.GetTransform` self) "Undefined" "MultiplyWithRoot" null null))
  (`KismetSystemLibrary.PrintString` (`KismetSystemLibrary.GetDisplayName` _returnvalue))
  (set `self.Time` 5.0)
  (`/Engine/EditorBlueprintResources/StandardMacros.IncrementInt` (`self.SpawnCount`)
    (:`  `
      (if (== (`self.SpawnCount`) 3)
        (set `self.Class` "/Game/Hamkt/Enemy/BP_EnemyRange.BP_EnemyRange_C")
        (if (== (`self.SpawnCount`) 5)
          (`KismetSystemLibrary.K2_ClearAndInvalidateTimerHandle` (`self.TH_MonsterTimerHandle`)))))))

(fn `UserConstructionScript`)