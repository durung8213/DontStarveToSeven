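; Weapon projectile actor that damages player characters it touches.
; On sphere overlap, only the authority acts, passing fixed damage to a BP_TestBasePlayerCharacter through TakeDamageMessage and ignoring other actors.
; After a hit it removes its particle component, stops projectile movement, spawns a Gideon end-burst emitter and destroys itself, each stage nested behind component validity checks.
; The impact emitter spawns inside the authority branch, with no multicast.
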(event `self.ReceiveBeginPlay`)

(event `self.Sphere.OnComponentBeginOverlap`
  (params (OverlappedComponent :type "PrimitiveComponent Object Reference") (OtherActor :type "Actor Object Reference") (OtherComp :type "PrimitiveComponent Object Reference") (OtherBodyIndex :type Integer) (bFromSweep :type Boolean) (SweepResult :type "HitResult Structure (by ref)"))
  (`/Engine/EditorBlueprintResources/ActorMacros.Switch Has Authority`
    (:`Authority`
      (bind _asbp_test_base_player_character (cast `/Game/Kimmh/Character/BP_TestBasePlayerCharacter` OtherActor))
      (message `BPI_EnemyAI.TakeDamage` _asbp_test_base_player_character 7.0 self)
      (bind _particlesystem (`self.ParticleSystem`)
        (:`then`
          (`ActorComponent.K2_DestroyComponent` _particlesystem)
          (bind _projectilemovement1 (`self.ProjectileMovement1`)
            (:`then`
              (`MovementComponent.StopMovementImmediately` _projectilemovement1)
              (`GameplayStatics.SpawnEmitterAtLocation` "/Game/Hamkt/RangeSkill/FX/Particles/Gideon/Abilities/Burden/FX/P_Gideon_Burden_DoT2_End.P_Gideon_Burden_DoT2_End" (`self.K2_GetActorLocation`) (struct) (2.0 2.0 2.0))
              (`self.StaticMesh`
                (:`then`
                  (`self.K2_DestroyActor`))
                (:`else`)))
            (:`else`)))
        (:`else`)))))

(fn `UserConstructionScript`)