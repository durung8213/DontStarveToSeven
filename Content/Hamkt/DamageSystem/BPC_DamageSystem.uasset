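; BPC_DamageSystem is a component that manages an actor's health, death, healing and incoming damage.
; TakeDamage runs a DamageInfo through the CanBeDamaged macro, which checks death, invincibility and blocking to block, apply or ignore the hit.
; Results go out through OnBlocked, OnDeath and OnDamageResponse dispatchers, the last firing only when interruptible or forced.
; Heal adds health clamped to MaxHealth while alive; a non-interrupting hit only prints a debug string.
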(fn `Heal`
  (params (Amount :type "Float (double-precision)"))
  (returns (NewHealth :type "Float (double-precision)"))
  (if (not (`self.bIsDead`))
    (bind _output_get (set `self.Health` (`KismetMathLibrary.FClamp` (+ Amount (`self.Health`)) 0.0 (`self.MaxHealth`))))
    (return _output_get)))

(fn `TakeDamage`
  (params (DamageInfo :type "/Game/Hamkt/DamageSystem/S_DamageInfo Structure"))
  (returns (WasDamaged :type Boolean))
  (bind (_amount _damagetype _damageresponse _shoulddamageinvincible _canbeblocked _canbeparried _shouldforceinterrupt) (break `/Game/Hamkt/DamageSystem/S_DamageInfo` DamageInfo))
  (`self.CanBeDamaged` _shoulddamageinvincible _canbeblocked ; 해당 매크로에서 확인
    (:`BlockDamage`
      (`self.OnBlocked` _canbeparried) ; 데미지를 차단
      (return true))
    (:`DoDamage`
      (bind _output_get (set `self.Health` (- (`self.Health`) _amount)))
      (if (<= _output_get 0.0)
        (set `self.bIsDead` true)
        (`self.OnDeath`) ; 죽으면 이벤트디스패처 호출
        (return true)
        (elif (or (`self.bIsInterruptible`) _shouldforceinterrupt)
          (`self.OnDamageResponse` _damageresponse)
          (return true)
          (else
            (`KismetSystemLibrary.PrintString` "Damae No")))))
    (:`NoDamage`
      (return false))))