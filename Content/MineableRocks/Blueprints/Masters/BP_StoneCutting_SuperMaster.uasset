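; Master Blueprint for a mineable rock that swaps itself for a breakable version when struck by a pickaxe.
; It shows OriginalStaticMesh, set in both construction and BeginPlay, until a BP_PickAxe overlaps the mesh.
; On authority only, it spawns RockToSpawn at its own transform, passes its class through an exposed-on-spawn StonecuttingSuperMaster parameter, then destroys itself.
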(event `self.ReceiveBeginPlay`
  (`StaticMeshComponent.SetStaticMesh` (`self.StaticMesh`) (`self.Original Static Mesh`)))

(event `self.StaticMesh.OnComponentBeginOverlap`
  (params (OverlappedComponent :type "PrimitiveComponent Object Reference") (OtherActor :type "Actor Object Reference") (OtherComp :type "PrimitiveComponent Object Reference") (OtherBodyIndex :type Integer) (bFromSweep :type Boolean) (SweepResult :type "HitResult Structure (by ref)"))
  (bind (_returnvalue_location _returnvalue_rotation _returnvalue_scale) (`KismetMathLibrary.BreakTransform` (`self.GetTransform`)))
  ;[1 1 1] Spawn actual chaos tree on overlap with character axe
  (cast `/Game/MineableRocks/MineableRocks_Character/Blueprints/BP_PickAxe` OtherActor)
  (`/Engine/EditorBlueprintResources/ActorMacros.Switch Has Authority`
    (:`Authority`
      (`|SpawnActorFromClass` (`self.Rock to spawn`) (`KismetMathLibrary.MakeTransform` _returnvalue_location _returnvalue_rotation _returnvalue_scale) "AlwaysSpawn" "SelectDefaultAtRuntime" null (`GameplayStatics.GetObjectClass` self) null)
      (`self.K2_DestroyActor`))))

(fn `UserConstructionScript`
  (`StaticMeshComponent.SetStaticMesh` (`self.StaticMesh`) (`self.Original Static Mesh`)))