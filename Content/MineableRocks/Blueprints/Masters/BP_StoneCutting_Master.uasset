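; Master Blueprint for a mineable rock that fractures with Chaos destruction, drops ores, and can respawn or self-destroy after inactivity.
; Point damage spawns damage-scaled impact fields on a geometry collection held by an anchor field and made dynamic at BeginPlay.
; Server-side break events accumulate mass, spawning ores at even thresholds.
; The final threshold fires a cluster strain field, removes the geometry and starts actor cleanup; any base mesh then becomes damageable.
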(event `Play Sound On Clients`
  (params (Sound :type "SoundBase Object Reference"))
  ;[1 1 1] Multicast break sound to clients and spawn sound at location
  (`GameplayStatics.PlaySoundAtLocation` Sound (`self.K2_GetActorLocation`) (struct) 1.0 1.0 0.0 null null null null))

(event `Destroy geometry`
  ;[1 1 1] Logic for letting object break
  (`KismetSystemLibrary.Delay` (`self.Delay before fractures are destroyed after meeting threshold`))
  (`ActorComponent.K2_DestroyComponent` (`self.GeometryCollection`))
  (`ActorComponent.K2_DestroyComponent` (`self.CollionCapsuleForOres`))
  (`ActorComponent.K2_DestroyComponent` (`self.BP_Chaos_AnchorField`))
  (`ActorComponent.K2_DestroyComponent` (`self.BP_Chaos_ClusterStrainField`)))

(event `self.GeometryCollection.OnChaosBreakEvent`
  (params (BreakEvent :type "ChaosBreakEvent Structure (by ref)"))
  ;[1 1 1] Logic for letting object break
  (`/Engine/EditorBlueprintResources/ActorMacros.Switch Has Authority`
    (:`Authority`
      (`self.Calculate mass chopped and check if has met threshold to spawn ore` BreakEvent)
      (if (>= (`self.Total Mass Broken`) (`self.Mass required to be chopped before breaking`))
        (`/Engine/EditorBlueprintResources/StandardMacros.DoOnce` false
          (:`Completed`
            (set `self.Has broken` true)
            (`self.Play Sound On Clients` (`self.Break Sound`))
            (bind _asbp_chaos_cluster_strain_field (cast `/Game/ResourcePack/Chaos/BP_Chaos_ClusterStrainField` (`ChildActorComponent.ChildActor` (`self.BP_Chaos_ClusterStrainField`))))
            (`/Game/ResourcePack/Chaos/BP_Chaos_ClusterStrainField.Activate Clusterstrainfield` _asbp_chaos_cluster_strain_field)
            (`|ExecutionSequence`
              (:`then_0`
                (`self.Destroy geometry`))
              (:`then_1`
                (`self.Destroy Cutting Actor`)))))))))

(event `self.ReceivePointDamage`
  (params (Damage :type "Float (single-precision)") (DamageType :type "DamageType Object Reference") (HitLocation :type "Vector Structure") (HitNormal :type "Vector Structure") (HitComponent :type "PrimitiveComponent Object Reference") (BoneName :type Name) (ShotFromDirection :type "Vector Structure") (InstigatedBy :type "Controller Object Reference") (DamageCauser :type "Actor Object Reference") (HitInfo :type "HitResult Structure (by ref)"))
  (bind _returnvalue (+ (* Damage 0.01) 1.0))
  ;[1 1 1] On damage
  ;;[1 1 1] This checks if it is the trunk that is hit and if it may be hit. If so, calculate trunk logic, if not, do nothing.
  (`self.Base Mesh Logic` HitComponent Damage)
  (`|SpawnActorFromClass` "/Game/ResourcePack/Chaos/BP_Chaos_WeaponImpact.BP_Chaos_WeaponImpact_C" (`KismetMathLibrary.MakeTransform` (`.Location` (`GameplayStatics.BreakHitResult` HitInfo))) "Undefined" "MultiplyWithRoot" null (* (* 25000.0 _returnvalue) (`self.Force Mutliplier`)) (* (* 1.35 _returnvalue) (`self.Force Mutliplier`)) true null))

(event `Destroy Cutting Actor`
  ;[1 1 1] Destroy the treecutting actor by event
  (if (`self.Does Respawn`)
    ;;[1 1 1] Check if we should not respawn when trunk is destroyed, and check IF the trunk is destroyed. If so, don't respawn and destroy actor
    (if (`self.When base mesh is destroyed do not respawn`)
      (if (not (`self.Base Mesh is destroyed`))
        ;;[1 1 1] Waiting for respawn
        (`KismetSystemLibrary.Delay` (`self.Respawn time`) :!label _label)
        (set `self.Respawn Timer is active` true)
        (`|SpawnActorFromClass` (`self.Stonecutting Super Master`) (`self.GetTransform`) "AlwaysSpawn" "SelectDefaultAtRuntime" null (`GameplayStatics.GetObjectClass` self) (`self.Original Static Mesh`) null))
      (else
        (goto _label)))
    (`self.K2_DestroyActor`)
    (else
      (`KismetSystemLibrary.Delay` (`self.Delay to destroy actor if not respawning`))
      (`self.K2_DestroyActor`))))

(event `Start inactivity timer`
  ;[1 1 1] Destroys actor after inactivity
  (`/Engine/EditorBlueprintResources/StandardMacros.DoOnce` false
    (:`Completed`
      (`KismetSystemLibrary.Delay` (`self.MaxInactivity`))
      ;;[1 1 1] If the respawn timer is active OR is in the process of breaking, just let it be. If not, destroy the actor
      (if (not (or (`self.Respawn Timer is active`) (`self.Has broken`)))
        (`self.K2_DestroyActor`)))))

(event `Set Dynamic`
  (bind _geometrycollection (`self.GeometryCollection`))
  (bind (_origin _boxextent _sphereradius) (`KismetSystemLibrary.GetComponentBounds` _geometrycollection))
  ;[1 1 1] When spawning the object dynamicly, the construction script does not seem to be excecuted properly and the anchor does not work. The geometry will move unless it is static. So we made the geometry static by default, and make it dynamic on begin play
  ;;[1 1 1] The "Set Dynamic" node sometimes makes a sphere that is larger than the geometry. So when it was set as dynamic it immediately falls through the world as it has no remaining static pieces to anchor the parts that are set as dynamic.  Try making that set dynamic size smaller to test. If it falls through, change the bounds and multiply by .a lower value to ensure the sphere size for the set bounds always leaves some as static for the anchor.
  (`GeometryCollectionComponent.ApplyKinematicField` _geometrycollection (* _sphereradius 0.75) (`KismetMathLibrary.MakeVector_NetQuantize` (.x _origin) (.y _origin) (+ (.z _origin) 25.0))))

(event `self.ReceiveBeginPlay`
  (`|ExecutionSequence`
    (:`then_0`
      ;[1 1 1] When spawning the object dynamicly, the construction script does not seem to be excecuted properly and the anchor does not work. The geometry will move unless it is static. So we made the geometry static by default, and make it dynamic on begin play
      ;;[1 1 1] Add the Anchorfield to the initialization field of the Chaos Gemeometry Collection. This makes sure it is "Anchored" and does not fall, etc.
      (bind `_as필드_시스템_액터` (cast `FieldSystemActor` (`ChildActorComponent.ChildActor` (`self.BP_Chaos_AnchorField`))))
      (`KismetArrayLibrary.Array_Add` (`GeometryCollectionComponent.InitializationFields` (`self.GeometryCollection`)) `_as필드_시스템_액터`)
      (`self.Set Dynamic`))
    (:`then_1`
      ;[1 1 1] Start inactivity timer
      (`self.Start inactivity timer`))
    (:`then_2`
      ;[1 1 1] Set base mesh if used
      (if (`self.Spawn Base Mesh`)
        (`StaticMeshComponent.SetStaticMesh` (`self.Base_Mesh`) (`self.Original Static Mesh`))))))

(fn `Base Mesh Logic`
  (params (A :type "Object Object Reference") (Damage :type "Float (double-precision)"))
  ;[1 1 1] I would prefer to use an CHAOS based trunk. However I do not seem to be able to set the "Object State" dynamicly. This is a proper alternative for now.
  ;;[1 1 1] Check if the trunk is hit, if so, destroy it
  (if (and (== A (`self.Base_Mesh`)) (`self.Has broken`))
    ;;[1 1 1] If trunk has met damage threshold, destroy the trunk component and call the destroy treeecutting actor
    (bind _met_damage_threshold (`self.Calculate damage done to trunk` Damage))
    (if _met_damage_threshold
      (set `self.Base Mesh is destroyed` true)
      ;;[1 1 1] Spawn item when trunk is destroyed
      (if (`self.Spawn item when base mesh is destroyed`)
        (`|SpawnActorFromClass` (`self.Spawn this item when base is destroyed`) (`SceneComponent.K2_GetComponentToWorld` (`self.Base_Mesh`)) "AdjustIfPossibleButAlwaysSpawn" "SelectDefaultAtRuntime" null null)
        ;;[1 1 1] Spawn trunk sound
        (`GameplayStatics.PlaySoundAtLocation` (`self.Base Mesh destruct sound`) (`self.K2_GetActorLocation`) (struct) 1.0 1.0 0.0 null null null null))
      (`ActorComponent.K2_DestroyComponent` (`self.Base_Mesh`))
      (`self.Destroy Cutting Actor`))))

(fn `Calculate Break Layers`
  ;[1 1 1] E.g.
  ; Total mass to be break down = 10
  ; Total ores = 5
  ; Fraction per ore spawn = 2
  ; Thresholds =  Ore spawn index * Fraction
  ;    1* 2 =2
  ;    2*2 = 4
  ;    3*2 = 6
  ;    etc.
  (for _index (range 1 (+ (`self.Amount of ores to spawn`) 1))
    (`KismetArrayLibrary.Array_Add` (`self.Spawn ore Thresholds`) (* (`self.Fraction off mass required to an ore to spawn`) (`KismetMathLibrary.Conv_IntToDouble` _index)))))

(fn `Calculate damage done to trunk`
  (params (Damage :type "Float (double-precision)"))
  (returns (`Met damage threshold` :type Boolean))
  (bind _output_get (set `self.Damage done to base Mesh` (+ (`self.Damage done to base Mesh`) Damage)))
  (`self.Calculate Break Layers`)
  (return (>= _output_get (`self.Damage required to destroy base mesh`))))

(fn `Calculate mass chopped and check if has met threshold to spawn ore`
  (params (ChaosBreakEvent :type "ChaosBreakEvent Structure (by ref)"))
  (bind ((`Component` _component) (`Location` _location) (`Extents` _extents) (`Mass` _mass)) (break `ChaosBreakEvent` ChaosBreakEvent))
  ;[1 1 1] Get mass from break event and add it to total mass variable
  (bind _output_get (set `self.Total Mass Broken` (+ (`self.Total Mass Broken`) _mass)))
  ;[1 1 1] Optionally print total mass chopped down
  (if (`self.Print Mass Chopped Down`)
    (`KismetSystemLibrary.PrintString` (`KismetStringLibrary.Concat_StrStr` "Total mass chopped down: " (`KismetStringLibrary.Conv_DoubleToString` _output_get)) true true (struct :`G` 0.66 :`B` 1.0 :`A` 1.0) 5.0))
  ;[1 1 1] check if total mass broken has met threshold value to spawn ore
  (if (>= (`self.Total Mass Broken`) (`self. Current mass required to spawn ore`))
    ;[1 1 1] When a threshold is met, reculculate  new mass required to spawn an ore
    (set `self. Current mass required to spawn ore` (+ (`self. Current mass required to spawn ore`) (`self.Fraction off mass required to an ore to spawn`)))
    ;[1 1 1] Check if the maximum of ores has been spawned
    (if (not (>= (`self.Ores spawned`) (`self.Amount of ores to spawn`)))
      ;[1 1 1] Spawn an ore at the break location
      (`|SpawnActorFromClass` (`self.Ore to Spawn`) (`KismetMathLibrary.MakeTransform` (+ _location (10.0 10.0 250.0))) "AdjustIfPossibleButAlwaysSpawn" "SelectDefaultAtRuntime" null null)
      (`self.Play Sound On Clients` (`self.Break Sound`))
      ;[1 1 1] Increment amount of ores spawned
      (set `self.Ores spawned` (+ (`self.Ores spawned`) 1))
      (return)
      (else
        (return)))
    (else
      (return))))

(fn `UserConstructionScript`
  (`|ExecutionSequence`
    (:`then_0`
      (bind _output_get (set `self.Fraction off mass required to an ore to spawn` (/ (`self.Mass required to be chopped before breaking`) (`KismetMathLibrary.Conv_IntToDouble` (`self.Amount of ores to spawn`)))))
      (set `self. Current mass required to spawn ore` _output_get))
    (:`then_1`
      (`self.Calculate Break Layers`)
      (if (`self.Print Threshold calucalation`)
        (for (_array_element _array_index) (`self.Spawn ore Thresholds`)
          (`KismetSystemLibrary.PrintString` (`KismetStringLibrary.Concat_StrStr` "Threshold Calculations: \nIndex: " (`KismetStringLibrary.Conv_IntToString` _array_index) "Threshold: " (`KismetStringLibrary.Conv_DoubleToString` _array_element)) true true (struct :`G` 0.66 :`B` 1.0 :`A` 1.0) 10.0))))))