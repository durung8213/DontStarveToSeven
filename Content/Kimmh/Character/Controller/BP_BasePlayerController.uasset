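; Base player controller that sets game-only input and handles interaction prompts, item pickup forwarding and a move-to-interactable action.
; Interaction hit results yield widget messages from hit actors, which are passed to ShowWidgetClient when valid.
; AddItem forwards items and their inventory type to InventoryComponent.
; The X key chains ServerMove into MultiMove, named as server-to-multicast calls, which uses SimpleMoveToLocation toward a valid InteractionActor.
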(event `self.ReceiveBeginPlay`
  (`WidgetBlueprintLibrary.SetInputMode_GameOnly` self))

(event `self.InteractionActorAction`
  (params (ResultArr :type "Array of HitResult Structure (by ref)"))
  (for _array_element ResultArr
    (bind _returnvalue (message `DTS_BPIInteraction.GetBaseInteractionWidget` (`.HitActor` (`GameplayStatics.BreakHitResult` _array_element))))
    (`/Engine/EditorBlueprintResources/StandardMacros.IsValid` _returnvalue
      (:`Is Valid`
        (`self.ShowWidgetClient` _returnvalue)))))

(event `AddItem`
  (params (InItem :type "Inventory Structure (by ref)") (InventoryType :type "EInventoryType Enum" :default "None"))
  (`SHInventoryComponent.AddItem` (`self.InventoryComponent`) InItem InventoryType))

(event `Key|X`
  (params (Key :type "Key Structure"))
  (:`Pressed`
    (`self.ServerMove`)))

(event `ServerMove`
  (`self.MultiMove`))

(event `MultiMove`
  (bind _interactionactor (`self.InteractionActor`)
    (:`then`
      (`AIBlueprintHelperLibrary.SimpleMoveToLocation` self (`self.K2_GetActorLocation` _interactionactor)))
    (:`else`)))

(fn `UserConstructionScript`)