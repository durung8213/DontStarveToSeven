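; Test player character Blueprint that binds debug keys to try out damage, wood-axe attack montages and effects.
; Keys call Server- and Multi-named events to damage itself, play AM_Resource swing sections, or spawn an explosion and damage BP_EnemyBossFirst.
; BeginPlay spawns a BP_Actor as TestActor, but the line-trace logic that moves it is disconnected.
; Other unwired experiments cover axe traces, weapon overlays, attachment, HP setting and attack toggling.
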(event `self.ReceiveTick`
  (params (DeltaSeconds :type "Float (single-precision)")))

(event `self.ReceiveBeginPlay`
  (bind _returnvalue (`|SpawnActorFromClass` "/Game/Kimmh/Blueprint/Test/BP_Actor.BP_Actor_C" (`KismetMathLibrary.MakeTransform` (0.0 0.0 0.0)) "Undefined" "MultiplyWithRoot" null null))
  (set `self.TestActor` _returnvalue))

(event `Key|Six`
  (params (Key :type "Key Structure"))
  (:`Pressed`
    (`self.ServerExtraSetCurrentHp`)))

(event `ServerExtraSetCurrentHp`
  (`self.TakeDamage` 20.0))

(event `TestServerEvent`)

(event `Key|Seven`
  (params (Key :type "Key Structure"))
  (:`Pressed`
    (`self.TestServerEvent`)))

(event `Key|Z`
  (params (Key :type "Key Structure"))
  (:`Pressed`
    (`self.ServerMontagePlayWithSession` "/Game/Kimmh/Character/Animation/AM/AM_Resource.AM_Resource" "WoodAxeSwing1" 1.0)))

(event `Key|Y`
  (params (Key :type "Key Structure"))
  (:`Pressed`
    (`self.ServerMontagePlayWithSession` "/Game/Kimmh/Character/Animation/AM/AM_Resource.AM_Resource" "WoodAxeSwing2" 1.0)))

(event `Key|C`
  (params (Key :type "Key Structure"))
  (:`Pressed`
    (`self.ServerMontagePlayWithSession` "/Game/Kimmh/Character/Animation/AM/AM_Resource.AM_Resource" "WoodAxeSwing3" 1.0)))

(event `Key|Seven`
  (params (Key :type "Key Structure"))
  (:`Pressed`
    (`self.ServerAex`)))

(event `MultiAex`
  (bind _returnvalue (`SkeletalMeshComponent.GetAnimInstance` (`self.Mesh`)))
  (`AnimInstance.Montage_Play` _returnvalue "/Game/Kimmh/Character/Animation/AM/AM_Resource.AM_Resource" 1.0 "MontageLength" 0.0 true)
  (`AnimInstance.Montage_JumpToSection` _returnvalue "WoodSwingFull" "/Game/Kimmh/Character/Animation/AM/AM_Resource.AM_Resource"))

(event `ServerAex`
  (`self.MultiAex`))

(event `self.CapsuleComponent.OnComponentBeginOverlap`
  (params (OverlappedComponent :type "PrimitiveComponent Object Reference") (OtherActor :type "Actor Object Reference") (OtherComp :type "PrimitiveComponent Object Reference") (OtherBodyIndex :type Integer) (bFromSweep :type Boolean) (SweepResult :type "HitResult Structure (by ref)")))

(event `MultiX`
  (bind _returnvalue (`GameplayStatics.GetActorOfClass` "/Game/Hamkt/Enemy/Boss/BP_EnemyBossFirst.BP_EnemyBossFirst_C"))
  (`GameplayStatics.SpawnEmitterAtLocation` "/Game/StarterContent/Particles/P_Explosion.P_Explosion")
  (`BPI_EnemyAI.TakeDamage` _returnvalue 20.0 null))

(event `Key|J`
  (params (Key :type "Key Structure"))
  (:`Pressed`
    (`self.MultiX`)))

(fn `ResetComboAttack`
  (set `self.ComboCount` 0))

(fn `UserConstructionScript`)