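; BP_NewBasePlayerCharacter is a player character Blueprint that spawns a BP_Actor at the world origin on BeginPlay and stores the reference in Actor2.
; Tick, overlap and construction script are empty.
; Disconnected nodes hold unfinished line-trace experiments from the player view point or camera child actor, plus a call to move Actor2, none of which run.
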(event `self.ReceiveBeginPlay`
  (bind _returnvalue (`|SpawnActorFromClass` "/Game/Kimmh/Blueprint/Test/BP_Actor.BP_Actor_C" (`KismetMathLibrary.MakeTransform` (0.0 0.0 0.0)) "Undefined" "MultiplyWithRoot" null null))
  (set `self.Actor2` _returnvalue))

(event `self.ReceiveTick`
  (params (DeltaSeconds :type "Float (single-precision)")))

(fn `UserConstructionScript`)