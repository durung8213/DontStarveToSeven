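; Test base weapon actor that deals melee-style hit damage through a Capsule overlap.
; On BeginPlay it stores its parent actor as owner so the capsule ignores that actor.
; AttackStart and AttackStop open and close the hit window, and overlaps during it send a fixed TakeDamage message on authority only.
; A hit-actor array limits damage to once per target per attack and clears on AttackStop.
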(event `self.ReceiveBeginPlay`
  (bind _returnvalue (`self.GetParentActor`))
  (`/Engine/EditorBlueprintResources/StandardMacros.IsValid` _returnvalue
    (:`Is Valid`
      (set `self.OwnerActor` _returnvalue))))

(event `self.Capsule.OnComponentBeginOverlap`
  (params (OverlappedComponent :type "PrimitiveComponent Object Reference") (OtherActor :type "Actor Object Reference") (OtherComp :type "PrimitiveComponent Object Reference") (OtherBodyIndex :type Integer) (bFromSweep :type Boolean) (SweepResult :type "HitResult Structure (by ref)"))
  (if (!= OtherActor (`self.OwnerActor`))
    (`/Engine/EditorBlueprintResources/ActorMacros.Switch Has Authority`
      (:`Authority`
        (if (`self.bCanAttack`)
          (if (not (`KismetArrayLibrary.Array_Contains` (`self.HitActorArr`) OtherActor))
            (message `BPI_EnemyAI.TakeDamage` OtherActor 20.0)
            (`KismetArrayLibrary.Array_Add` (`self.HitActorArr`) OtherActor)))))))

(event `AttackStart`
  (set `self.bCanAttack` true))

(event `AttackStop`
  (set `self.bCanAttack` false)
  (`KismetArrayLibrary.Array_Clear` (`self.HitActorArr`)))

(fn `UserConstructionScript`)