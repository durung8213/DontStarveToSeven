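; BP_TestInteraction is a test interactable that carries a WBP_BaseInteratcion prompt in its Widget component.
; BeginPlay casts the component's widget and collapses it, so the prompt starts hidden.
; GetInteractionWidget returns that cast widget to callers.
; GetInteractorData, ShowWidgetForPlayer and GetBaseInteractionWidget are empty stubs, so nothing in this Blueprint shows the prompt again.
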(event `self.ReceiveBeginPlay`
  (bind _aswbp_base_interatcion (cast `/Game/Kimmh/UI/Interaction/WBP_BaseInteratcion` (`WidgetComponent.GetWidget` (`self.Widget`))))
  (`Widget.SetVisibility` _aswbp_base_interatcion "Collapsed"))

(fn `GetBaseInteractionWidget`
  (returns (ReturnValue :type "DTS_BaseInteractionUserWidget Object Reference"))
  (return null))

(fn `GetInteractionWidget`
  (returns (RetrunWidget :type "/Game/Kimmh/UI/Interaction/WBP_BaseInteratcion Object Reference"))
  (bind _aswbp_base_interatcion (cast `/Game/Kimmh/UI/Interaction/WBP_BaseInteratcion` (`WidgetComponent.GetWidget` (`self.Widget`))))
  (return _aswbp_base_interatcion))

(fn `GetInteractorData`)

(fn `Show Widget for Player`
  (params (TargetPlayer :type "/Game/Kimmh/Character/Controller/BP_BasePlayerController Object Reference")))

(fn `UserConstructionScript`)